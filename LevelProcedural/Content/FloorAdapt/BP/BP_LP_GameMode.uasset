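; Game Mode for a simple top-down game that owns the UI widget, scoring and NPC population count.
; Creates WBP_TopDownUI_Action on BeginPlay and forwards item-use, score and combo changes to it.
; Score gains are multiplied by a combo that builds with repeated scoring and steps down after a retriggerable cooldown.
; Tracks the NPC count through increase/decrease events and reports whether spawning is allowed under the cap.
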(event `self.ReceiveBeginPlay`
  ;[0.15 0.15 0.15 0.502] As this is a very simple game, we're managing the UI from the Game Mode rather than a dedicated HUD actor
  (bind _returnvalue (`|CreateWidget` "/Game/Variant_TwinStick/UI/WBP_TopDownUI_Action.WBP_TopDownUI_Action_C" (`GameplayStatics.GetPlayerController` 0)))
  (bind _output_get (set `self.UI Widget` _returnvalue))
  (`UserWidget.AddToViewport` _output_get 0))

(event `self.ItemUsed`
  (params (NewValue :type Integer))
  ;[0.15 0.15 0.15 0.502] As this is a very simple game, we're managing the UI from the Game Mode rather than a dedicated HUD actor
  (`/Game/Variant_TwinStick/Blueprints/BPI_Twinstick.ItemUsed` (`self.UI Widget`) NewValue))

(event `self.ScoreUpdate`
  (params (NewValue :type Integer))
  ;[0.15 0.15 0.15 0.502] Scoring System - uses a simple combo multiplier with cooldown.
  (bind _output_get (set `self.Score` (+ (`self.Score`) (* (`self.Combo`) NewValue))))
  (`/Game/Variant_TwinStick/Blueprints/BPI_Twinstick.ScoreUpdate` (`self.UI Widget`) _output_get)
  (`self.ComboManager`))

(event `ComboManager`
  ;[0.15 0.15 0.15 0.502] Scoring System - uses a simple combo multiplier with cooldown.
  (`|ExecutionSequence`
    (:`then_0`
      (bind _result (`/Engine/EditorBlueprintResources/StandardMacros.IncrementInt` (`self.ComboIncrement`))
        (:`  `
          (if (and (> _result (`self.ComboIncrementMax`)) (<= (`self.Combo`) (`self.ComboCap`)))
            (bind _result_2 (`/Engine/EditorBlueprintResources/StandardMacros.IncrementInt` (`self.Combo`))
              (:`  `
                (`/Game/Variant_TwinStick/UI/WBP_TopDownUI_Action.ComboUpdate` (`self.UI Widget`) _result_2)
                (set `self.ComboIncrement` 0)))))))
    (:`then_1`
      (`KismetSystemLibrary.RetriggerableDelay` (`self.ComboCooldown`) :!label _label)
      (if (> (`self.Combo`) 1)
        (bind _result_3 (`/Engine/EditorBlueprintResources/StandardMacros.DecrementInt` (`self.Combo`))
          (:`  `
            (`/Game/Variant_TwinStick/UI/WBP_TopDownUI_Action.ComboUpdate` (`self.UI Widget`) _result_3)
            (set `self.ComboIncrement` 0)
            (`self.ComboTimer`)))))))

(event `ComboTimer`
  ;[0.15 0.15 0.15 0.502] Scoring System - uses a simple combo multiplier with cooldown.
  (goto _label))

(event `Increase NPCs`
  ; Manage NPC counts on the level
  (`/Engine/EditorBlueprintResources/StandardMacros.IncrementInt` (`self.Current NPC Count`)))

(event `Decrease NPCs`
  ; Manage NPC counts on the level
  (`/Engine/EditorBlueprintResources/StandardMacros.DecrementInt` (`self.Current NPC Count`)))

(fn `Should Spawn NPCs`
  (returns (Spawn :type Boolean))
  (return (<= (`self.Current NPC Count`) (`self.Max NPC Cap`))))

(fn `UserConstructionScript`)