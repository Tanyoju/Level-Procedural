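; BP_LP_Projectile is a short-lived projectile actor that deals damage to what it hits.
; On hit, it skips actors whose class is exactly BP_LP_Character; otherwise it applies damage, credited to the first player controller, and destroys itself.
; It also destroys itself when its projectile movement stops or when the lifespan set on spawn expires.
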(event `self.ReceiveBeginPlay`
  ; On spawn, set Projectile to destroy itself after 2 seconds
  (`self.SetLifeSpan` 2.0))

(event `self.ReceiveHit`
  (params (MyComp :type "PrimitiveComponent Object Reference") (Other :type "Actor Object Reference") (OtherComp :type "PrimitiveComponent Object Reference") (bSelfMoved :type Boolean) (HitLocation :type "Vector Structure") (HitNormal :type "Vector Structure") (NormalImpulse :type "Vector Structure") (Hit :type "HitResult Structure (by ref)"))
  ; If Hit, send a Projectile Impact message to the hit actor. If hit actor is a Top Down NPC, destroy self.
  (if (not (== (`GameplayStatics.GetObjectClass` Other) "/Game/FloorAdapt/BP/Character/BP_LP_Character.BP_LP_Character_C"))
    (`GameplayStatics.ApplyDamage` Other (`self.Damage`) (`GameplayStatics.GetPlayerController` 0) self "/Script/Engine.DamageType")
    (`self.K2_DestroyActor`)))

(event `self.ProjectileMovement.OnProjectileStop`
  (params (ImpactResult :type "HitResult Structure (by ref)"))
  ; Destroy self if Projectile stops moving
  (`self.K2_DestroyActor`))

(fn `UserConstructionScript`)