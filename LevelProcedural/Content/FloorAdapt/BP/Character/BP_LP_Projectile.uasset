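; Projectile Blueprint that damages enemies on hit and cleans itself up.
; A hit applies its damage, credited to player controller 0, prints a debug string and destroys the projectile.
; This only runs when the hit actor's class exactly equals BP_LP_EnemyParent, so child classes do not match.
; Otherwise it is destroyed when its movement component stops or its short lifespan, set on BeginPlay, expires.
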(event `self.ReceiveBeginPlay`
  ; On spawn, set Projectile to destroy itself after 2 seconds
  (`self.SetLifeSpan` 2.0))

(event `self.ReceiveHit`
  (params (MyComp :type "PrimitiveComponent Object Reference") (Other :type "Actor Object Reference") (OtherComp :type "PrimitiveComponent Object Reference") (bSelfMoved :type Boolean) (HitLocation :type "Vector Structure") (HitNormal :type "Vector Structure") (NormalImpulse :type "Vector Structure") (Hit :type "HitResult Structure (by ref)"))
  ; If Hit, send a Projectile Impact message to the hit actor. If hit actor is a Top Down NPC, destroy self.
  (if (== (`GameplayStatics.GetObjectClass` Other) "/Game/FloorAdapt/BP/Enemy/BP_LP_EnemyParent.BP_LP_EnemyParent_C")
    (`KismetSystemLibrary.PrintString` "Hello" true false (struct :`R` 1.0 :`G` 0.165365 :`B` 0.037677 :`A` 1.0) 5.0)
    (`GameplayStatics.ApplyDamage` Other (`self.Damage`) (`GameplayStatics.GetPlayerController` 0) null "/Script/Engine.DamageType")
    (`self.K2_DestroyActor`)))

(event `self.ProjectileMovement.OnProjectileStop`
  (params (ImpactResult :type "HitResult Structure (by ref)"))
  ; Destroy self if Projectile stops moving
  (`self.K2_DestroyActor`))

(fn `UserConstructionScript`)