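; Base enemy Blueprint that pursues the player and serves as a parent for attack variants.
; On BeginPlay it runs AI MoveTo toward the player, then calls an empty Attack event on reaching attack range.
; Damage reduces HP until Death tells the game mode whether a projectile killed it, spawns a destruction actor, then destroys itself and its first attached actor.
; Construction creates a dynamic enemy material instance.
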(event `self.ReceiveBeginPlay`
  (set `self.CurrentHP` (`self.MaxHP`))
  (`self.Move`))

(event `Move`
  (`|AIMoveTo` self (0.0 0.0 0.0) (`GameplayStatics.GetPlayerCharacter` 0) (`self.AttackRange`)
    (:`OnSuccess`
      (`KismetSystemLibrary.PrintString` "Success" true false (struct :`G` 0.66 :`B` 1.0 :`A` 1.0) 5.0)
      (`self.Attack`))))

(event `self.ReceiveAnyDamage`
  (params (Damage :type "Float (single-precision)") (DamageType :type "DamageType Object Reference") (InstigatedBy :type "Controller Object Reference") (DamageCauser :type "Actor Object Reference"))
  (bind _output_get (set `self.CurrentHP` (- (`self.CurrentHP`) Damage)))
  (if (<= _output_get 0.0)
    (set `self.DeathCause` DamageCauser)
    (`self.Death`)))

(event `Death`
  (bind _output (`|GetArrayItem` (`self.GetAttachedActors` true)))
  (`|ExecutionSequence`
    (:`then_0`
      (bind _asbp_lp_game_mode (cast `/Game/FloorAdapt/BP/BP_LP_GameMode` (`GameplayStatics.GetGameMode`)))
      (`/Game/FloorAdapt/BP/BP_LP_GameMode.Decrease NPCs` _asbp_lp_game_mode (== (`GameplayStatics.GetObjectClass` (`self.DeathCause`)) "/Game/FloorAdapt/BP/Character/BP_LP_Projectile.BP_LP_Projectile_C")))
    (:`then_1`
      (`|SpawnActorFromClass` "/Game/Variant_TwinStick/Blueprints/AI/BP_TwinStickNPCDestruction.BP_TwinStickNPCDestruction_C" (`SceneComponent.K2_GetComponentToWorld` (`self.Mesh`)) "Undefined" "MultiplyWithRoot" null null)
      (`self.SetActorHiddenInGame` true)
      (`self.SetActorEnableCollision` false)
      (`KismetSystemLibrary.Delay` 0.1)
      (`/Engine/EditorBlueprintResources/StandardMacros.IsValid` _output
        (:`Is Valid`
          (`self.K2_DestroyActor` _output))
        (:`Is Not Valid`
          _))
      (`self.K2_DestroyActor`))))

(event `Attack`)

(fn `UserConstructionScript`
  (bind _returnvalue (`PrimitiveComponent.CreateDynamicMaterialInstance` (`self.StaticMesh`) 0 "/Game/FloorAdapt/BP/Enemy/MI_Enemy.MI_Enemy" "None"))
  (set `self.MI_Enemy` _returnvalue))