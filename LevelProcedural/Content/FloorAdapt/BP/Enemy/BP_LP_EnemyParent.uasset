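; Base enemy Blueprint that walks to the player, attacks, takes damage and dies.
; BeginPlay fills health and issues a single AI MoveTo toward the player, calling the empty Attack event on arrival within attack range, presumably for child classes to override.
; Incoming damage reduces health; at zero, Death spawns a TwinStick destruction actor at the mesh transform, hides the enemy, disables collision and destroys it shortly after.
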(event `self.ReceiveBeginPlay`
  (set `self.CurrentHP` (`self.MaxHP`))
  (`|AIMoveTo` self (0.0 0.0 0.0) (`GameplayStatics.GetPlayerCharacter` 0) (`self.AttackRange`)
    (:`OnSuccess`
      (`KismetSystemLibrary.PrintString` "Success" true false (struct :`G` 0.66 :`B` 1.0 :`A` 1.0) 5.0)
      (`self.Attack`))))

(event `Attack`)

(event `self.ReceiveAnyDamage`
  (params (Damage :type "Float (single-precision)") (DamageType :type "DamageType Object Reference") (InstigatedBy :type "Controller Object Reference") (DamageCauser :type "Actor Object Reference"))
  (bind _output_get (set `self.CurrentHP` (- (`self.CurrentHP`) Damage)))
  (if (<= _output_get 0.0)
    (`self.Death`)))

(event `Death`
  (`|SpawnActorFromClass` "/Game/Variant_TwinStick/Blueprints/AI/BP_TwinStickNPCDestruction.BP_TwinStickNPCDestruction_C" (`SceneComponent.K2_GetComponentToWorld` (`self.Mesh`)) "Undefined" "MultiplyWithRoot" null null)
  (`self.SetActorHiddenInGame` true)
  (`self.SetActorEnableCollision` false)
  (`KismetSystemLibrary.Delay` 0.1)
  (`self.K2_DestroyActor`))

(fn `UserConstructionScript`)