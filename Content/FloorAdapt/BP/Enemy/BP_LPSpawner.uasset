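; BP_LPSpawner is an NPC spawner that releases groups of a configurable class at random reachable navmesh points within a radius.
; On BeginPlay it finds the RecastNavMesh, retrying until valid, spawns a first group and starts a looping timer.
; Each timer tick resets the group counter and spawns again if BP_TwinStickGameMode allows it.
; SpawnNPC calls itself through a DoN gate with short random delays to stagger each group.
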(event `self.ReceiveBeginPlay`
  ;[0.15 0.15 0.15 0.502] Reference the Navmesh and start Spawning
  (`|ExecutionSequence`
    (:`then_0`
      (`self.Find Nav Mesh`))
    (:`then_1`
      (`self.Spawn NPC`))
    (:`then_3`
      (`KismetSystemLibrary.K2_SetTimerDelegate` (delegate `Spawn Timer Expired`) (`self.SpawnDelay`) true))))

(event `Find Nav Mesh`
  ;[0.15 0.15 0.15 0.502] Find the navmesh and store a reference
  (bind _outactors (`GameplayStatics.GetAllActorsOfClass` "/Script/NavigationSystem.RecastNavMesh"))
  (bind _output (`|GetArrayItem` _outactors))
  (`/Engine/EditorBlueprintResources/StandardMacros.IsValid` _output
    (:`Is Valid`
      (set `self.NavData` _output))
    (:`Is Not Valid`
      (`KismetSystemLibrary.Delay` 0.2)
      (`self.Find Nav Mesh`))))

(event `Spawn Timer Expired`
  ;[0.15 0.15 0.15 0.502] Logic to spawn NPCs when a timer expires. The spawner checks if we're at the Max Cap first so we don't overshoot our NPC limit and then spawns an NPC.
  (`self.Reset Spawn Group`)
  (bind _asbp_twin_stick_game_mode (cast `/Game/Variant_TwinStick/Blueprints/BP_TwinStickGameMode` (`GameplayStatics.GetGameMode`)))
  (if (`/Game/Variant_TwinStick/Blueprints/BP_TwinStickGameMode.Should Spawn NPCs` _asbp_twin_stick_game_mode)
    (`self.Spawn NPC`)))

(event `Spawn NPC`
  (bind (_randomlocation _returnvalue) (`NavigationSystemV1.K2_GetRandomReachablePointInRadius` (`self.K2_GetActorLocation`) (`self.SpawnRadius`) (`self.NavData`) null))
  ;[0.15 0.15 0.15 0.502] Logic to spawn NPCs when a timer expires. The spawner checks if we're at the Max Cap first so we don't overshoot our NPC limit and then spawns an NPC.
  (bind _counter (`/Engine/EditorBlueprintResources/StandardMacros.Do N` (`self.SpawnGroupSize`) :!label _label) ; Run the Spawn Logic until we've\nspawned the desired amount of\nNPCs
    (:`Exit`
      (if _returnvalue
        (`|SpawnActorFromClass` (`self.Spawn Class`) (`KismetMathLibrary.Conv_VectorToTransform` _randomlocation) "AdjustIfPossibleButAlwaysSpawn" "MultiplyWithRoot" null null)
        (if (< _counter (`self.SpawnGroupSize`))
          (`KismetSystemLibrary.Delay` (`KismetMathLibrary.RandomFloatInRange` 0.33 0.66))
          (`self.Spawn NPC`))))))

(event `Reset Spawn Group`
  ;[0.15 0.15 0.15 0.502] Logic to spawn NPCs when a timer expires. The spawner checks if we're at the Max Cap first so we don't overshoot our NPC limit and then spawns an NPC.
  (goto _label :!via `Reset`))

(fn `UserConstructionScript`)