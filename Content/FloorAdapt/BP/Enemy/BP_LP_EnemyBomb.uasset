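; BP_LP_EnemyBomb is a bomb enemy that damages the player when its explosion wind-up completes.
; Attack plays a timeline that drives the Alpha parameter on the enemy's material.
; When it finishes, the first BP_LP_Character still overlapping the Sphere takes Damage and a debug "BOOOM" prints.
; The character leaving the Sphere reverses the explosion timeline and calls Move.
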(event `self.Attack`
  (bind _output (`|GetArrayItem` (`PrimitiveComponent.GetOverlappingActors` (`self.Sphere`) "/Game/FloorAdapt/BP/Character/BP_LP_Character.BP_LP_Character_C")))
  ; Enemy explodes when player is near
  (bind (_direction _newtrack_0) (`Timeline|T_Explosion`)
    (:`Update`
      (`MaterialInstanceDynamic.SetScalarParameterValue` (`self.MI_Enemy`) "Alpha" _newtrack_0))
    (:`Finished`
      (`/Engine/EditorBlueprintResources/StandardMacros.IsValid` _output
        (:`Is Valid`
          (`GameplayStatics.ApplyDamage` _output (`self.Damage`))
          (`KismetSystemLibrary.PrintString` "BOOOM" true false (struct :`R` 1.0 :`G` 0.034947 :`A` 1.0)))))))

(event `self.Sphere.OnComponentEndOverlap`
  (params (OverlappedComponent :type "PrimitiveComponent Object Reference") (OtherActor :type "Actor Object Reference") (OtherComp :type "PrimitiveComponent Object Reference") (OtherBodyIndex :type Integer))
  (if (== (`GameplayStatics.GetObjectClass` OtherActor) "/Game/FloorAdapt/BP/Character/BP_LP_Character.BP_LP_Character_C")
    (`TimelineComponent.Reverse` (`self.T_Explosion`))
    (`self.Move`)))

(fn `UserConstructionScript`
  (`parent.UserConstructionScript`))