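; Shield-carrying enemy that makes melee attacks against the player character BP_LP_Character.
; On BeginPlay it spawns a BP_Shield actor, snaps it onto ShieldPlacement, then after a short delay overrides the movement component's rotation rate.
; Attack applies Damage to the first character overlapping its Sphere, then calls Move whether or not anything was hit.
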(event `self.ReceiveBeginPlay`
  (`parent.ReceiveBeginPlay`)
  (bind _returnvalue (`|SpawnActorFromClass` "/Game/FloorAdapt/BP/Enemy/BP_Shield.BP_Shield_C" (`KismetMathLibrary.MakeTransform` (0.0 0.0 0.0)) "Undefined" "MultiplyWithRoot" null null))
  (`self.K2_AttachToComponent` _returnvalue (`self.ShieldPlacement`) "None" "SnapToTarget" "SnapToTarget" "SnapToTarget" true)
  (`KismetSystemLibrary.Delay` 0.5)
  (set `CharacterMovementComponent.RotationRate` (struct :`Yaw` 50.0) (`self.CharacterMovement`)))

(event `self.Attack`
  (bind _output (`|GetArrayItem` (`PrimitiveComponent.GetOverlappingActors` (`self.Sphere`) "/Game/FloorAdapt/BP/Character/BP_LP_Character.BP_LP_Character_C")))
  (`/Engine/EditorBlueprintResources/StandardMacros.IsValid` _output
    (:`Is Valid`
      (`GameplayStatics.ApplyDamage` _output (`self.Damage`)))
    (:`Is Not Valid`
      _))
  (`self.Move`))

(fn `UserConstructionScript`
  (`parent.UserConstructionScript`))