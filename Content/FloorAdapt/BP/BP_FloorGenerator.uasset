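; Procedural floor actor that builds a randomized grid of mesh tiles with gaps when GenerateRandomFloor is triggered.
; The event randomizes scale, power and seed, clears the HISM, then lays tiles spaced by mesh bounds wherever power-shaped 2D Perlin noise passes a threshold.
; Rows at both ends of the grid always stay solid.
; BeginPlay and the construction script generate nothing, and the GenerateHISM row helper is not called here.
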(event `self.ReceiveBeginPlay`)

(event `GenerateRandomFloor`
  (params (MinScale :type "Float (double-precision)") (MaxScale :type "Float (double-precision)") (MinPower :type "Float (double-precision)") (MaxPower :type "Float (double-precision)"))
  (bind _rowindex (`self.RowIndex`))
  (bind (_cubesize_x _cubesize_y) (`KismetMathLibrary.BreakVector` (`self.CubeSize`)))
  (bind (_returnvalue_min _returnvalue_max) (break `Box` (`StaticMesh.GetBoundingBox` (`StaticMeshComponent.StaticMesh` (`self.HierarchicalInstancedStaticMesh`)))))
  (set `self.Scale` (`KismetMathLibrary.RandomFloatInRange` MinScale MaxScale))
  (set `self.Power` (`KismetMathLibrary.RandomFloatInRange` MinPower MaxPower))
  (set `self.Seed` (`KismetMathLibrary.RandomIntegerInRange` 0 10000))
  (`InstancedStaticMeshComponent.ClearInstances` (`self.HierarchicalInstancedStaticMesh`))
  (set `self.CubeSize` (- _returnvalue_max _returnvalue_min))
  (for _index (range (+ (`self.N_Row`) 1))
    (set `self.RowIndex` _index)
    (for _index_2 (range (+ (`self.N_Column`) 1))
      (set `self.ColumnIndex` _index_2)
      (if (or (> (`KismetMathLibrary.MultiplyMultiply_FloatFloat` (`KismetMathLibrary.MapRangeClamped` (`SimpleNoiseGeneratorsBPLibrary.PerlinNoise2D` (`KismetMathLibrary.Conv_IntToDouble` _rowindex) (`KismetMathLibrary.Conv_IntToDouble` (`self.ColumnIndex`)) (`self.Scale`) (`self.Cell Size`) 0.0 (`self.Seed`)) -1.0 1.0 0.0 1.0) (`self.Power`)) 0.5) (<= _rowindex 1) (>= _rowindex (- (`self.N_Row`) 1)))
        (`InstancedStaticMeshComponent.AddInstance` (`self.HierarchicalInstancedStaticMesh`) (`KismetMathLibrary.MakeTransform` (`KismetMathLibrary.MakeVector` (* (`self.RowIndex`) _cubesize_x) (* (`self.ColumnIndex`) _cubesize_y))) false)))))

(fn `GenerateHISM`
  (bind (_cubesize_x _cubesize_y) (`KismetMathLibrary.BreakVector` (`self.CubeSize`)))
  (for _index (range 25)
    (set `self.ColumnIndex` _index)
    (`InstancedStaticMeshComponent.AddInstance` (`self.HierarchicalInstancedStaticMesh`) (`KismetMathLibrary.MakeTransform` (`KismetMathLibrary.MakeVector` (* (`self.RowIndex`) _cubesize_x) (* (`self.ColumnIndex`) _cubesize_y))) false :!label _label))
  (for _index_2 (range 1 26)
    (set `self.ColumnIndex` (* _index_2 -1))
    (goto _label)))

(fn `UserConstructionScript`)