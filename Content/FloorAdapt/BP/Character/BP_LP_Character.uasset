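; Twin-stick player character that moves, aims, fires projectiles, dashes, uses AoE items and has a debug-drawn sword trace.
; Tick snaps yaw to the cursor hit in mouse mode, or interpolates toward the stick angle.
; Gamepad and touch inputs share logic, with aiming driving delay-throttled auto-fire and a DoOnce gating item use.
; Damage lowers and prints health, while projectile impacts launch the player and run a Timeline-driven global time dilation.
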(event `self.ReceiveTick`
  (params (DeltaSeconds :type "Float (single-precision)"))
  (bind (_bblockinghit _binitialoverlap _time _distance _location) (`GameplayStatics.BreakHitResult` (`PlayerController.GetHitResultUnderCursorByChannel` (`GameplayStatics.GetPlayerController` 0) "TraceTypeQuery1" true)))
  (bind (_returnvalue_roll _returnvalue_pitch _returnvalue_yaw) (`KismetMathLibrary.BreakRotator` (`KismetMathLibrary.FindLookAtRotation` (`self.K2_GetActorLocation`) _location)))
  ;[0.15 0.15 0.15 0.502] Player Rotation is handled on Tick, meaning it updates every frame. The Mouse input snaps the Player to the correct facing, the Gamepad smoothly interpolates.
  (if (`PlayerController.bShowMouseCursor` (`GameplayStatics.GetPlayerController` 0))
    (if _bblockinghit
      (set `self.Target Rotation` _returnvalue_yaw)
      (`self.SnapPlayerToFacing`))
    (else
      (`self.RotatePlayer`))))

(event `self.ReceiveBeginPlay`
  ;[0.15 0.15 0.15 0.502] Setup Input Mapping & Items
  (`EnhancedInputSubsystemInterface.AddMappingContext` (pcsubsystem `EnhancedInputLocalPlayerSubsystem` (`GameplayStatics.GetPlayerController` 0)) "/Game/FloorAdapt/Input/IMC_LP.IMC_LP" 0 (struct))
  (message `/Game/Variant_TwinStick/Blueprints/BPI_Twinstick.ItemUsed` (`GameplayStatics.GetGameMode`) (`self.Items`))
  (set `self.CurrentHealth` (`self.MaxHealth`)))

(event `EnhancedInput|/Game/FloorAdapt/Input/Actions/IA_LP_MouseAim`
  (params (ActionValue :type "Vector2D Structure") (ElapsedSeconds :type "Float (double-precision)") (TriggeredSeconds :type "Float (double-precision)") (InputAction :type "InputAction Object Reference" :default "/Game/FloorAdapt/Input/Actions/IA_LP_MouseAim.IA_LP_MouseAim"))
  ;[0.15 0.15 0.15 0.502] If Player moves the mouse, enable mouse controls.
  (:`Triggered`
    (set `PlayerController.bShowMouseCursor` true (`GameplayStatics.GetPlayerController` 0))))

(event `EnhancedInput|/Game/FloorAdapt/Input/Actions/IA_LP_Fire`
  (params (ActionValue :type Boolean) (ElapsedSeconds :type "Float (double-precision)") (TriggeredSeconds :type "Float (double-precision)") (InputAction :type "InputAction Object Reference" :default "/Game/FloorAdapt/Input/Actions/IA_LP_Fire.IA_LP_Fire"))
  (bind (_returnvalue_location _returnvalue_rotation _returnvalue_scale) (`KismetMathLibrary.BreakTransform` (`self.GetTransform`)))
  ;[0.15 0.15 0.15 0.502] Fire projectile in Player's facing direction
  (:`Triggered`
    (`|SpawnActorFromClass` "/Game/FloorAdapt/BP/Character/BP_LP_Projectile.BP_LP_Projectile_C" (`KismetMathLibrary.MakeTransform` (+ (`KismetMathLibrary.GreaterGreater_VectorRotator` (`KismetMathLibrary.MakeVector` (`self.Projectile Offset`)) _returnvalue_rotation) _returnvalue_location) _returnvalue_rotation _returnvalue_scale) "Undefined" "MultiplyWithRoot" null null :!label _label)))

(event `EnhancedInput|/Game/FloorAdapt/Input/Actions/IA_LP_Move`
  (params (ActionValue :type "Vector2D Structure") (ElapsedSeconds :type "Float (double-precision)") (TriggeredSeconds :type "Float (double-precision)") (InputAction :type "InputAction Object Reference" :default "/Game/FloorAdapt/Input/Actions/IA_LP_Move.IA_LP_Move"))
  ;[0.15 0.15 0.15 0.502] Move the Player and control their aiming direction if on a Gamepad
  (:`Triggered`
    (`self.Move` ActionValue_X ActionValue_Y)))

(event `Reset Item`
  ;[0.15 0.15 0.15 0.502] If the Player has a smart bomb, fire it when the Use Item input action is called.
  (goto _label_3 :!via `Reset`))

(event `AutoFire`
  ;[0.15 0.15 0.15 0.502] Fire projectile in Player's facing direction
  (goto _label))

(event `EnhancedInput|/Game/FloorAdapt/Input/Actions/IA_LP_UseItem`
  (params (ActionValue :type Boolean) (ElapsedSeconds :type "Float (double-precision)") (TriggeredSeconds :type "Float (double-precision)") (InputAction :type "InputAction Object Reference" :default "/Game/FloorAdapt/Input/Actions/IA_LP_UseItem.IA_LP_UseItem"))
  ;[0.15 0.15 0.15 0.502] If the Player has a smart bomb, fire it when the Use Item input action is called.
  (:`Triggered`
    (if (> (`self.Items`) 0) :!label _label_2
      (`/Engine/EditorBlueprintResources/StandardMacros.DoOnce` false :!label _label_3
        (:`Completed`
          (`|ExecutionSequence`
            (:`then_0`
              (`|SpawnActorFromClass` "/Game/Variant_TwinStick/Blueprints/BP_TwinStickAoEAttack.BP_TwinStickAoEAttack_C" (`KismetMathLibrary.Conv_VectorToTransform` (`self.K2_GetActorLocation`)) "Undefined" "MultiplyWithRoot" null null)
              (`KismetSystemLibrary.Delay` 1.0)
              (`self.Reset Item`))
            (:`then_1`
              (`/Engine/EditorBlueprintResources/StandardMacros.DecrementInt` (`self.Items`)
                (:`  `
                  (message `/Game/Variant_TwinStick/Blueprints/BPI_Twinstick.ItemUsed` (`GameplayStatics.GetGameMode`) (`self.Items`) :!label _label_4))))))))))

(event `self.Primary Thumbstick`
  (params (Axis :type "Vector2D Structure"))
  ;[0.15 0.15 0.15 0.502] Move the Player and control their aiming direction if on a Gamepad
  (`self.Move` Axis_Y Axis_X))

(event `self.Touch Item Start`
  ;[0.15 0.15 0.15 0.502] If the Player has a smart bomb, fire it when the Use Item input action is called.
  (goto _label_2))

(event `EnhancedInput|/Game/FloorAdapt/Input/Actions/IA_LP_StickAim`
  (params (ActionValue :type "Vector2D Structure") (ElapsedSeconds :type "Float (double-precision)") (TriggeredSeconds :type "Float (double-precision)") (InputAction :type "InputAction Object Reference" :default "/Game/FloorAdapt/Input/Actions/IA_LP_StickAim.IA_LP_StickAim"))
  ;[0.15 0.15 0.15 0.502] Move the Player and control their aiming direction if on a Gamepad
  (:`Triggered`
    (`self.StickAim` ActionValue_X ActionValue_Y)
    (if (not (`self.AutoFireActive`)) :!label _label_5
      (set `self.AutoFireActive` true)
      (`self.AutoFire`)
      (`KismetSystemLibrary.Delay` (`self.AutoFireDelay`))
      (set `self.AutoFireActive` false))))

(event `EnhancedInput|/Game/FloorAdapt/Input/Actions/IA_LP_SwordAttack`
  (params (ActionValue :type Boolean) (ElapsedSeconds :type "Float (double-precision)") (TriggeredSeconds :type "Float (double-precision)") (InputAction :type "InputAction Object Reference" :default "/Game/FloorAdapt/Input/Actions/IA_LP_SwordAttack.IA_LP_SwordAttack"))
  (bind _returnvalue (`self.K2_GetActorLocation`))
  ;[0.15 0.15 0.15 0.502] Fire projectile in Player's facing direction
  (:`Triggered`
    (`MovementComponent.StopMovementImmediately` (`self.CharacterMovement`))
    (`KismetSystemLibrary.SphereTraceSingle` :`Start` _returnvalue :`End` (+ _returnvalue (* (`self.GetActorForwardVector`) (`self.SwordRange`))) :`Radius` 50.0 :`TraceChannel` "TraceTypeQuery1" :`DrawDebugType` "ForDuration")))

(event `self.Secondary Thumbstick`
  (params (Axis :type "Vector2D Structure"))
  ;[0.15 0.15 0.15 0.502] Move the Player and control their aiming direction if on a Gamepad
  (`self.TouchAim` Axis_Y Axis_X)
  (goto _label_5))

(event `self.Interaction`
  (params (Interactor :type "Actor Object Reference"))
  ;[0.15 0.15 0.15 0.502] If an Item sends an interaction message to the Player, add an Item to the inventory
  (if (== (`GameplayStatics.GetObjectClass` Interactor) "/Game/Variant_TwinStick/Blueprints/BP_TwinStickPickup.BP_TwinStickPickup_C")
    (`/Engine/EditorBlueprintResources/StandardMacros.IncrementInt` (`self.Items`)
      (:`  `
        (goto _label_4)))))

(event `EnhancedInput|/Game/FloorAdapt/Input/Actions/IA_LP_Dash`
  (params (ActionValue :type Boolean) (ElapsedSeconds :type "Float (double-precision)") (TriggeredSeconds :type "Float (double-precision)") (InputAction :type "InputAction Object Reference" :default "/Game/FloorAdapt/Input/Actions/IA_LP_Dash.IA_LP_Dash"))
  (bind (_returnvalue_x _returnvalue_y) (`KismetMathLibrary.BreakVector2D` (`|GetInputActionValue`)))
  ;[0.15 0.15 0.15 0.502] Dash
  (:`Triggered`
    (`self.LaunchCharacter` (* (`KismetMathLibrary.MakeVector` (`KismetMathLibrary.FClamp` _returnvalue_x -1.0) (`KismetMathLibrary.FClamp` _returnvalue_y -1.0)) 2500.0) true true :!label _label_6)))

(event `self.ReceiveAnyDamage`
  (params (Damage :type "Float (single-precision)") (DamageType :type "DamageType Object Reference") (InstigatedBy :type "Controller Object Reference") (DamageCauser :type "Actor Object Reference"))
  ; Damaged
  (bind _output_get (set `self.CurrentHealth` (- (`self.CurrentHealth`) Damage)))
  (`KismetSystemLibrary.PrintString` (`KismetStringLibrary.Conv_DoubleToString` _output_get) true false (struct :`R` 0.0435 :`G` 1.0 :`A` 1.0) 5.0))

(event `self.Touch Dash Start`
  ;[0.15 0.15 0.15 0.502] Dash
  (goto _label_6))

(event `self.ProjectileImpact`
  (params (ForwardVector :type "Vector Structure"))
  ;[0.15 0.15 0.15 0.502] Knock Back Player
  (`self.LaunchCharacter` (* (`KismetMathLibrary.MakeVector` ForwardVector_X ForwardVector_Y) (`self.KnockbackStrength`)) true true)
  ;[0.15 0.15 0.15 0.502] Dilate Time via a Timeline
  (bind (_direction _timedilation) (`Timeline|Timeline` :!via `PlayFromStart`)
    (:`Update`
      (`GameplayStatics.SetGlobalTimeDilation` _timedilation))
    (:`Finished`
      (`GameplayStatics.SetGlobalTimeDilation` 1.0))))

(fn `Move`
  (params (`Axis X` :type "Float (double-precision)") (`Axis Y` :type "Float (double-precision)"))
  (bind (_returnvalue_roll _returnvalue_pitch _returnvalue_yaw) (`KismetMathLibrary.BreakRotator` (`self.GetControlRotation`)))
  (bind (_returnvalue_roll_2 _returnvalue_pitch_2 _returnvalue_yaw_2) (`KismetMathLibrary.BreakRotator` (`self.GetControlRotation`)))
  (`self.AddMovementInput` (`KismetMathLibrary.GetForwardVector` (`KismetMathLibrary.MakeRotator` _returnvalue_roll 0.0 _returnvalue_yaw)) `Axis X`)
  (`self.AddMovementInput` (`KismetMathLibrary.GetRightVector` (`KismetMathLibrary.MakeRotator` _returnvalue_roll_2 0.0 _returnvalue_yaw_2)) `Axis Y`))

(fn `RotatePlayer`
  (bind (_returnvalue_roll _returnvalue_pitch _returnvalue_yaw) (`KismetMathLibrary.BreakRotator` (`self.K2_GetActorRotation`)))
  (bind (_returnvalue_roll_2 _returnvalue_pitch_2 _returnvalue_yaw_2) (`KismetMathLibrary.BreakRotator` (`KismetMathLibrary.RInterpTo` (`self.K2_GetActorRotation`) (`KismetMathLibrary.MakeRotator` _returnvalue_roll _returnvalue_pitch (`self.Target Rotation`)) (`GameplayStatics.GetWorldDeltaSeconds`) 10.0)))
  (if (not (`KismetMathLibrary.NearlyEqual_FloatFloat` _returnvalue_yaw (`self.Target Rotation`) 0.5))
    (`self.K2_SetActorRotation` (`KismetMathLibrary.MakeRotator` _returnvalue_roll _returnvalue_pitch _returnvalue_yaw_2))
    (return)))

(fn `SnapPlayerToFacing`
  (bind (_returnvalue_roll _returnvalue_pitch) (`KismetMathLibrary.BreakRotator` (`self.K2_GetActorRotation`)))
  (`self.K2_SetActorRotation` (`KismetMathLibrary.MakeRotator` _returnvalue_roll _returnvalue_pitch (`self.Target Rotation`)))
  (return))

(fn `StickAim`
  (params (`Axis X` :type "Float (double-precision) (by ref)") (`Axis Y` :type "Float (double-precision)"))
  (bind _result (`/Engine/EditorBlueprintResources/StandardMacros.NegateFloat` `Axis X`)
    (:`  `
      (set `self.Target Rotation` (`KismetMathLibrary.DegAtan2` `Axis Y` _result))
      (set `PlayerController.bShowMouseCursor` false (`GameplayStatics.GetPlayerController` 0)))))

(fn `TouchAim`
  (params (`Axis X` :type "Float (double-precision) (by ref)") (`Axis Y` :type "Float (double-precision)"))
  (set `self.Target Rotation` (`KismetMathLibrary.DegAtan2` `Axis Y` `Axis X`))
  (set `PlayerController.bShowMouseCursor` false (`GameplayStatics.GetPlayerController` 0)))

(fn `UserConstructionScript`)