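; Elevator actor that carries the floor-to-floor transition, with sliding double doors.
; A character entering the box saves walked distance and health to the game mode, triggers floor generation, resets distance and closes the doors, which reopen once shut; exiting closes them again.
; Timelines drive the doors and a MoveElevatorUp event that lifts the actor one floor, then opens them.
; Reposition, fade and wave-start logic is left unwired.
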(event `self.ReceiveBeginPlay`)

(event `self.Box.OnComponentEndOverlap`
  (params (OverlappedComponent :type "PrimitiveComponent Object Reference") (OtherActor :type "Actor Object Reference") (OtherComp :type "PrimitiveComponent Object Reference") (OtherBodyIndex :type Integer))
  (cast `/Game/FloorAdapt/BP/Character/BP_LP_Character` OtherActor)
  (`self.CloseDoors`))

(event `self.Box.OnComponentBeginOverlap`
  (params (OverlappedComponent :type "PrimitiveComponent Object Reference") (OtherActor :type "Actor Object Reference") (OtherComp :type "PrimitiveComponent Object Reference") (OtherBodyIndex :type Integer) (bFromSweep :type Boolean) (SweepResult :type "HitResult Structure (by ref)"))
  (bind _gamemoderef (`self.GameModeRef`))
  (bind _asbp_lp_character (cast `/Game/FloorAdapt/BP/Character/BP_LP_Character` OtherActor))
  (`/Game/FloorAdapt/BP/BP_LP_GameMode.SaveData` _gamemoderef (`/Game/FloorAdapt/BP/Character/BP_LP_Character.DistanceWalked` _asbp_lp_character) (`/Game/FloorAdapt/BP/Character/BP_LP_Character.CurrentHealth` _asbp_lp_character))
  (`/Game/FloorAdapt/BP/BP_LP_GameMode.GenerateFloor` _gamemoderef)
  (`self.CloseDoors`)
  (set `self.bool` true)
  (set `/Game/FloorAdapt/BP/Character/BP_LP_Character.DistanceWalked` 0 _asbp_lp_character))

(event `OpenDoors`
  (set `self.Reverse?` false)
  (bind (_direction _newtrack_0) (`Timeline|T_Doors` :!label _label)
    (:`Update`
      (`SceneComponent.K2_SetRelativeLocation` (`self.DoorLeft`) (`KismetMathLibrary.MakeVector` (`KismetMathLibrary.Lerp` 75.0 220.0 _newtrack_0) -140.0 20.0) false false)
      (`SceneComponent.K2_SetRelativeLocation` (`self.DoorRight`) (`KismetMathLibrary.MakeVector` (`KismetMathLibrary.Lerp` -75.0 -220.0 _newtrack_0) -140.0 20.0) false false))
    (:`Finished`
      (if (and (`self.Reverse?`) (`self.bool`))
        (`self.OpenDoors`)
        (set `self.bool` false)))))

(event `CloseDoors`
  (set `self.Reverse?` true)
  (goto _label :!via `Reverse`))

(event `MoveElevatorUp`
  (set `self.LocationBeforeMoving` (`self.K2_GetActorLocation`))
  (bind (_direction _newtrack_0) (`Timeline|T_Elevator` :!via `PlayFromStart`)
    (:`Update`
      (`self.K2_SetActorLocation` (`KismetMathLibrary.VLerp` (`self.LocationBeforeMoving`) (+ (`self.LocationBeforeMoving`) (0.0 0.0 1500.0)) _newtrack_0)))
    (:`Finished`
      (`self.OpenDoors`))))

(fn `UserConstructionScript`)