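; BP_FloorGenerator is an actor that builds a patchy floor grid from Hierarchical Instanced Static Mesh instances.
; Its construction script loops over rows and columns, spacing tiles by the mesh's bounding box and placing one only where seeded 2D Perlin noise is positive.
; GenerateHISM, uncalled here, lays a solid line of instances along Y on both sides of zero at the current row.
; The event graph holds only disconnected random-fill logic.
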(event `self.ReceiveBeginPlay`)

(fn `GenerateHISM`
  (bind (_cubesize_x _cubesize_y) (`KismetMathLibrary.BreakVector` (`self.CubeSize`)))
  (for _index (range 25)
    (set `self.ColumnIndex` _index)
    (`InstancedStaticMeshComponent.AddInstance` (`self.HierarchicalInstancedStaticMesh`) (`KismetMathLibrary.MakeTransform` (`KismetMathLibrary.MakeVector` (* (`self.RowIndex`) _cubesize_x) (* (`self.ColumnIndex`) _cubesize_y))) false :!label _label))
  (for _index_2 (range 1 26)
    (set `self.ColumnIndex` (* _index_2 -1))
    (goto _label)))

(fn `UserConstructionScript`
  (bind (_cubesize_x _cubesize_y) (`KismetMathLibrary.BreakVector` (`self.CubeSize`)))
  (bind (_returnvalue_min _returnvalue_max) (break `Box` (`StaticMesh.GetBoundingBox` (`StaticMeshComponent.StaticMesh` (`self.HierarchicalInstancedStaticMesh`)))))
  (set `self.CubeSize` (- _returnvalue_max _returnvalue_min))
  (for _index (range (+ (`self.N_Row`) 1))
    (bind _output_get (set `self.RowIndex` _index))
    (for _index_2 (range (+ (`self.N_Column`) 1))
      (bind _output_get_2 (set `self.ColumnIndex` _index_2))
      (if (> (`SimpleNoiseGeneratorsBPLibrary.PerlinNoise2D` (`KismetMathLibrary.Conv_IntToDouble` _output_get) (`KismetMathLibrary.Conv_IntToDouble` _output_get_2) (`self.Scale`) (`self.Cell Size`) 0.0 (`self.Seed`)) 0.0)
        (`InstancedStaticMeshComponent.AddInstance` (`self.HierarchicalInstancedStaticMesh`) (`KismetMathLibrary.MakeTransform` (`KismetMathLibrary.MakeVector` (* (`self.RowIndex`) _cubesize_x) (* (`self.ColumnIndex`) _cubesize_y))) false)))))