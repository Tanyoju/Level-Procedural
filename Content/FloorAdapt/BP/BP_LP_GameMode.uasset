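; Game Mode for a floor-based wave game that adapts enemy composition to the player's gun versus sword kills.
; It creates the UI and spawn manager, and forwards score with a decaying combo multiplier to the widget.
; Each cleared wave stores kills in a four-slot ring buffer and starts a larger one after a delay.
; Gun-heavy play brings mostly shield enemies, sword-heavy mostly bombers, balanced play a closer mix.
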(event `self.ReceiveBeginPlay`
  ;[0.15 0.15 0.15 0.502] As this is a very simple game, we're managing the UI from the Game Mode rather than a dedicated HUD actor
  (bind _returnvalue (`|CreateWidget` "/Game/Variant_TwinStick/UI/WBP_TopDownUI_Action.WBP_TopDownUI_Action_C" (`GameplayStatics.GetPlayerController` 0)))
  (bind _output_get (set `self.UI Widget` _returnvalue))
  (`UserWidget.AddToViewport` _output_get 0)
  (bind _returnvalue_2 (`|SpawnActorFromClass` "/Game/FloorAdapt/BP/Enemy/BP_SpawnManager.BP_SpawnManager_C" (`KismetMathLibrary.MakeTransform` (0.0 0.0 0.0)) "Undefined" "MultiplyWithRoot" null null))
  (set `self.SpawnManagerRef` _returnvalue_2)
  (`self.WaveStart`))

(event `self.ItemUsed`
  (params (NewValue :type Integer))
  ;[0.15 0.15 0.15 0.502] As this is a very simple game, we're managing the UI from the Game Mode rather than a dedicated HUD actor
  (`/Game/Variant_TwinStick/Blueprints/BPI_Twinstick.ItemUsed` (`self.UI Widget`) NewValue))

(event `self.ScoreUpdate`
  (params (NewValue :type Integer))
  ;[0.15 0.15 0.15 0.502] Scoring System - uses a simple combo multiplier with cooldown.
  (bind _output_get (set `self.Score` (+ (`self.Score`) (* (`self.Combo`) NewValue))))
  (`/Game/Variant_TwinStick/Blueprints/BPI_Twinstick.ScoreUpdate` (`self.UI Widget`) _output_get)
  (`self.ComboManager`))

(event `ComboManager`
  ;[0.15 0.15 0.15 0.502] Scoring System - uses a simple combo multiplier with cooldown.
  (`|ExecutionSequence`
    (:`then_0`
      (bind _result (`/Engine/EditorBlueprintResources/StandardMacros.IncrementInt` (`self.ComboIncrement`))
        (:`  `
          (if (and (> _result (`self.ComboIncrementMax`)) (<= (`self.Combo`) (`self.ComboCap`)))
            (bind _result_2 (`/Engine/EditorBlueprintResources/StandardMacros.IncrementInt` (`self.Combo`))
              (:`  `
                (`/Game/Variant_TwinStick/UI/WBP_TopDownUI_Action.ComboUpdate` (`self.UI Widget`) _result_2)
                (set `self.ComboIncrement` 0)))))))
    (:`then_1`
      (`KismetSystemLibrary.RetriggerableDelay` (`self.ComboCooldown`) :!label _label)
      (if (> (`self.Combo`) 1)
        (bind _result_3 (`/Engine/EditorBlueprintResources/StandardMacros.DecrementInt` (`self.Combo`))
          (:`  `
            (`/Game/Variant_TwinStick/UI/WBP_TopDownUI_Action.ComboUpdate` (`self.UI Widget`) _result_3)
            (set `self.ComboIncrement` 0)
            (`self.ComboTimer`)))))))

(event `ComboTimer`
  ;[0.15 0.15 0.15 0.502] Scoring System - uses a simple combo multiplier with cooldown.
  (goto _label))

(event `Decrease NPCs`
  (params (`KilledByGun?` :type Boolean))
  ; Manage NPC counts on the level
  (bind _result (`/Engine/EditorBlueprintResources/StandardMacros.DecrementInt` (`self.NumberOfEnnemiesInWave`))
    (:`  `
      (if `KilledByGun?`
        (`/Engine/EditorBlueprintResources/StandardMacros.IncrementInt` (`self.EnemyKilledWithGun`)
          (:`  `
            _))
        (else
          (`/Engine/EditorBlueprintResources/StandardMacros.IncrementInt` (`self.EnemyKilledWithSword`)
            (:`  `
              _))))
      (if (<= _result 0)
        (`self.WaveEnd`)
        (`KismetSystemLibrary.PrintString` "WAVE END" true false (struct :`R` 0.354723 :`B` 1.0 :`A` 1.0) 5.0)))))

(event `WaveEnd`
  ; Manage NPC counts on the level
  (`KismetArrayLibrary.Array_Set` (`self.GunKillsOnFloors`) (mod (`self.Floor`) 4) (`self.EnemyKilledWithGun`))
  (`KismetArrayLibrary.Array_Set` (`self.SwordKillsOnFloors`) (mod (`self.Floor`) 4) (`self.EnemyKilledWithSword`))
  (`/Engine/EditorBlueprintResources/StandardMacros.IncrementInt` (`self.Floor`)
    (:`  `
      (`KismetSystemLibrary.Delay` 5.0)
      (`self.WaveStart`))))

(event `WaveStart`
  (bind _bombenemiestospawn (`self.BombEnemiesToSpawn`))
  (bind _shieldenemiestospawn (`self.ShieldEnemiesToSpawn`))
  ; Manage NPC counts on the level
  (set `self.NumberOfEnnemiesInWave` (+ (* (`self.Floor`) 2) 6))
  (bind (_shieldenemies _bombenemies) (`self.DetermineEnemiesToSpawn`))
  (set `self.ShieldEnemiesToSpawn` _shieldenemies)
  (set `self.BombEnemiesToSpawn` _bombenemies)
  (`/Game/FloorAdapt/BP/Enemy/BP_SpawnManager.SetupWave` (`self.SpawnManagerRef`) _shieldenemiestospawn _bombenemiestospawn)
  (`KismetSystemLibrary.PrintString` (`KismetStringLibrary.Concat_StrStr` "WAVE START :: " "Shield :" (`KismetStringLibrary.Conv_IntToString` _shieldenemiestospawn) "  Bomb : " (`KismetStringLibrary.Conv_IntToString` _bombenemiestospawn)) true false (struct :`R` 0.354723 :`B` 1.0 :`A` 1.0) 5.0))

(fn `CalculateEnemiesOfLastXFloor`
  (params (NumberOfFloor :type Integer))
  (returns (TotalEnemies :type Integer))
  (locals (L_TotalEnemies :type Integer))
  (for _index (range 1 (+ NumberOfFloor 1))
    (set `local.L_TotalEnemies` (+ (`local.L_TotalEnemies`) (+ (* (- (`self.Floor`) _index) 2) 6))))
  (return (`self.NumberOfEnnemiesInWave`)))

(fn `DetermineEnemiesToSpawn`
  (returns (ShieldEnemies :type Integer) (BombEnemies :type Integer))
  (locals (L_TotalSwordKills :type Integer) (L_TotalGunKills :type Integer) (L_RandomLastIndex :type Integer :default 0) (L_ShieldToSpawn :type Integer) (L_BombToSpawn :type Integer))
  (set `local.L_RandomLastIndex` (`KismetMathLibrary.RandomIntegerInRange` 2 3))
  (for _index (range (+ (`local.L_RandomLastIndex`) 1))
    (set `local.L_TotalGunKills` (+ (`local.L_TotalGunKills`) (`|GetArrayItem` (`self.GunKillsOnFloors`) _index))))
  (for _index_2 (range (+ (`local.L_RandomLastIndex`) 1))
    (set `local.L_TotalSwordKills` (+ (`local.L_TotalSwordKills`) (`|GetArrayItem` (`self.SwordKillsOnFloors`) _index_2))))
  (if (<= (`KismetMathLibrary.Abs_Int` (- (`local.L_TotalGunKills`) (`local.L_TotalSwordKills`))) (/ (`self.CalculateEnemiesOfLastXFloor` (+ (`local.L_RandomLastIndex`) 1)) 4))
    (set `local.L_BombToSpawn` (`KismetMathLibrary.RandomIntegerInRange` (/ (`self.NumberOfEnnemiesInWave`) 3) (/ (`self.NumberOfEnnemiesInWave`) 2)))
    (set `local.L_ShieldToSpawn` (- (`self.NumberOfEnnemiesInWave`) (`local.L_BombToSpawn`)))
    (elif (> (`local.L_TotalGunKills`) (`local.L_TotalSwordKills`))
      (set `local.L_BombToSpawn` (`KismetMathLibrary.RandomIntegerInRange` 1 (/ (`self.NumberOfEnnemiesInWave`) 4)))
      (set `local.L_ShieldToSpawn` (- (`self.NumberOfEnnemiesInWave`) (`local.L_BombToSpawn`)))
      (else
        (set `local.L_ShieldToSpawn` (`KismetMathLibrary.RandomIntegerInRange` 1 (/ (`self.NumberOfEnnemiesInWave`) 4)))
        (set `local.L_BombToSpawn` (- (`self.NumberOfEnnemiesInWave`) (`local.L_ShieldToSpawn`))))))
  (return (`local.L_ShieldToSpawn`) (`local.L_BombToSpawn`)))

(fn `Should Spawn NPCs`
  (returns (Spawn :type Boolean))
  (return (<= (`self.Current NPC Count`) (`self.Max NPC Cap`))))

(fn `UserConstructionScript`)